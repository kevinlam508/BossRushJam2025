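; Player pawn Blueprint with an orbiting weapon that swings in an A or B variant, plus health and invincibility.
; Swing inputs drive OrbitingWeapon, whose events switch TypeCollision between A, B and neutral and spawn color-coded attached VFX with absolute rotation.
; Damage applies only outside invincibility, then starts it; Health events update a viewport health bar.
; BeginPlay also snaps Orion to the mesh's root_ship socket.
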(event `self.ReceiveEndPlay`
  (params (EndPlayReason :type "EEndPlayReason Enum" :default "Destroyed"))
  (`Widget.RemoveFromParent` (`self.HealthBar`)))

(event `self.ReceiveBeginPlay`
  (bind _returnvalue (`|CreateWidget` "/Game/Blueprints/UI/PlayerHealthBar.PlayerHealthBar_C"))
  (bind _output_get (set `self.HealthBar` _returnvalue))
  (`UserWidget.AddToViewport` _output_get 0)
  (`self.UpdateHealthBar` (`HealthComponent.CurrentHealth` (`self.Health`)))
  (`SceneComponent.K2_AttachToComponent` (`self.Orion`) (`self.Mesh`) "root_ship" "SnapToTarget" "KeepWorld" "KeepRelative" true))

(event `EnhancedInput|/Game/ThirdPerson/Input/Actions/IA_SwingA`
  (params (ActionValue :type Boolean) (ElapsedSeconds :type "Float (double-precision)") (TriggeredSeconds :type "Float (double-precision)") (InputAction :type "InputAction Object Reference" :default "/Game/ThirdPerson/Input/Actions/IA_SwingA.IA_SwingA"))
  (:`Started`
    (`OrbitingWeapon.SwingA` (`self.OrbitingWeapon`))))

(event `EnhancedInput|/Game/ThirdPerson/Input/Actions/IA_SwingB`
  (params (ActionValue :type Boolean) (ElapsedSeconds :type "Float (double-precision)") (TriggeredSeconds :type "Float (double-precision)") (InputAction :type "InputAction Object Reference" :default "/Game/ThirdPerson/Input/Actions/IA_SwingB.IA_SwingB"))
  (:`Started`
    (`OrbitingWeapon.SwingB` (`self.OrbitingWeapon`))))

(event `self.OrbitingWeapon.OnASwingBegin`
  (`TypeCollision.ToA` (`self.TypeCollision`))
  (`self.SpawnWeaponVFX` (struct :`G` 0.280113 :`B` 1.0 :`A` 1.0)))

(event `self.OrbitingWeapon.OnBSwingBegin`
  (`TypeCollision.ToB` (`self.TypeCollision`))
  (`self.SpawnWeaponVFX` (struct :`R` 1.0 :`A` 1.0) true))

(event `self.OrbitingWeapon.OnSwingEnd`
  (`TypeCollision.ToNeutral` (`self.TypeCollision`)))

(event `self.ReceiveAnyDamage`
  (params (Damage :type "Float (single-precision)") (DamageType :type "DamageType Object Reference") (InstigatedBy :type "Controller Object Reference") (DamageCauser :type "Actor Object Reference"))
  (bind _invincibility (`self.Invincibility`))
  (if (not (`InvincibilityComponent.GetIsInvincible` _invincibility))
    (`HealthComponent.TakeDamage` (`self.Health`) Damage)
    (`InvincibilityComponent.StartInvincibility` _invincibility)))

(event `self.Health.OnHeal`
  (params (Delta :type "Float (single-precision)") (NewValue :type "Float (single-precision)"))
  (`self.UpdateHealthBar` NewValue))

(event `self.Health.OnTakeDamage`
  (params (Delta :type "Float (single-precision)") (NewValue :type "Float (single-precision)"))
  (`self.UpdateHealthBar` NewValue))

(fn `SpawnWeaponVFX`
  (params (Color :type "LinearColor Structure") (IsB :type Boolean))
  (locals (SpawnedWeaponVFX :type "NiagaraComponent Object Reference"))
  (bind _spawnedweaponvfx (`local.SpawnedWeaponVFX`))
  (bind _returnvalue (`NiagaraFunctionLibrary.SpawnSystemAttached` (`self.Weapon VFX`) (`self.OrbitingWeapon`) "None" (0.0 0.0 0.0) (struct) "KeepRelativeOffset"))
  (bind _output_get (set `local.SpawnedWeaponVFX` _returnvalue))
  (`FXSystemComponent.SetColorParameter` _output_get "ParticleColor" Color)
  (`NiagaraComponent.SetVariableBool` _spawnedweaponvfx "IsB" IsB)
  (`SceneComponent.SetAbsolute` _spawnedweaponvfx false true false))

(fn `UpdateHealthBar`
  (params (NewValue :type "Float (double-precision)"))
  (`ProgressBar.SetPercent` (`/Game/Blueprints/UI/PlayerHealthBar.Bar` (`self.HealthBar`)) (`KismetMathLibrary.SafeDivide` NewValue (`HealthComponent.MaxHealth` (`self.Health`)))))

(fn `UserConstructionScript`)