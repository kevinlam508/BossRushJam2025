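; Boss3_BP is the third boss's actor, with a health component and an on-screen BossHealthBar widget that tracks damage and healing.
; Point damage on the main body reduces health.
; Hits on colliders under RotationColliders instead tell Boss3Controller to rotate a board corner, passing the hit collider's name and damage type.
; A toggle event from RotationColliderEvents shows or hides four cylinder meshes.
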(event `self.ReceiveEndPlay`
  (params (EndPlayReason :type "EEndPlayReason Enum" :default "Destroyed"))
  (`Widget.RemoveFromParent` (`self.HealthBar`)))

(event `self.ReceiveBeginPlay`
  (bind _returnvalue (`|CreateWidget` "/Game/Blueprints/UI/BossHealthBar.BossHealthBar_C"))
  (bind _output_get (set `self.HealthBar` _returnvalue))
  (`UserWidget.AddToViewport` _output_get 0)
  (`self.UpdateHealthBar` (`HealthComponent.CurrentHealth` (`self.Health`))))

(event `self.Health.OnTakeDamage`
  (params (Delta :type "Float (single-precision)") (NewValue :type "Float (single-precision)"))
  (`self.UpdateHealthBar` NewValue))

(event `self.Health.OnHeal`
  (params (Delta :type "Float (single-precision)") (NewValue :type "Float (single-precision)"))
  (`self.UpdateHealthBar` NewValue))

(event `self.ReceivePointDamage`
  (params (Damage :type "Float (single-precision)") (DamageType :type "DamageType Object Reference") (HitLocation :type "Vector Structure") (HitNormal :type "Vector Structure") (HitComponent :type "PrimitiveComponent Object Reference") (BoneName :type Name) (ShotFromDirection :type "Vector Structure") (InstigatedBy :type "Controller Object Reference") (DamageCauser :type "Actor Object Reference") (HitInfo :type "HitResult Structure (by ref)"))
  (if (== (`self.MainBodyRoot`) HitComponent)
    (`HealthComponent.TakeDamage` (`self.Health`) Damage)
    (elif (== (`self.RotationColliders`) (`SceneComponent.GetAttachParent` HitComponent))
      (bind _asboss_3controller (cast `Boss3Controller` (`AIBlueprintHelperLibrary.GetAIController` self)))
      (`Boss3Controller.RotateBoardCorner` _asboss_3controller (`KismetStringLibrary.Conv_StringToName` (`KismetSystemLibrary.GetObjectName` HitComponent)) (`GameplayStatics.GetObjectClass` DamageType)))))

(event `self.RotationColliderEvents.OnToggleRotationColliders`
  (params (On :type Boolean))
  (bind _returnvalue (not On))
  (`SceneComponent.SetHiddenInGame` (`self.Cylinder3`) _returnvalue false)
  (`SceneComponent.SetHiddenInGame` (`self.Cylinder1`) _returnvalue false)
  (`SceneComponent.SetHiddenInGame` (`self.Cylinder`) _returnvalue false)
  (`SceneComponent.SetHiddenInGame` (`self.Cylinder2`) _returnvalue false))

(fn `UpdateHealthBar`
  (params (NewValue :type "Float (double-precision)"))
  (`ProgressBar.SetPercent` (`/Game/Blueprints/UI/BossHealthBar.Bar` (`self.HealthBar`)) (`KismetMathLibrary.SafeDivide` NewValue (`HealthComponent.MaxHealth` (`self.Health`)))))

(fn `UserConstructionScript`)